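; Asteroid actor for a twin-stick game that teleports to a random edge of the camera's view on BeginPlay and tumbles as it moves.
; It estimates the view rectangle from camera FOV, aspect ratio and height above the floor, offset once by the player's starting position.
; A timeline drives roll and pitch, reissuing a five-second mesh move toward a second random perimeter point, passed as a relative location, each update.
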(event EventBeginPlay
  (CallFunction|GetMainCamera)
  (CallFunction|GetFOVDimensions)
  (CallFunction|GetFOVCorners)
  (bind _randposn (CallFunction|GetRandPointonPerim))
  (Transformation|SetActorLocation _randposn false true)
  (bind _randposn_2 (CallFunction|GetRandPointonPerim))
  (bind _x (Timeline|Rotation%20Timeline PlayFromStart)
    (:Update
      (Transformation|SetActorRelativeRotation (Math|Rotator|MakeRotator _x _x 0.0))
      (Components|MoveComponentTo (Variables|Default|GetStaticMesh) _randposn_2 (Math|Rotator|MakeRotator 0.0 0.0 0.0) false false 5.0 false))))

(event Collision|EventActorBeginOverlap
  (params (OtherActor :type Actor%20Object%20Reference)))

(event EventTick
  (params (DeltaSeconds :type Float%20%28single-precision%29)))

(fn ConstructionScript)

(fn GetMainCamera
  (bind _astwin_stick_pawn (Utilities|Casting|CastToTwinStickPawn (Game|Player|GetPlayerPawn 0))
    (:then
      (Variables|Default|SetCamera (Variables|/Game/TwinStickBP/Blueprints/TwinStickPawn.TwinStickPawn_C|GetCameraComponent _astwin_stick_pawn))
      ;[1 1 1] make sure this updates on tick
      (Variables|Default|SetPlayerLocation (Transformation|GetActorLocation _astwin_stick_pawn)))
    (:CastFailed
      (Development|PrintString "Whomst"))))

(fn GetFOVDimensions
  (bind _desiredview (Class|CameraComponent|GetCameraView (Variables|Default|GetCamera) 0.0))
  (Variables|Default|SetCameraLocation (.Location (Utilities|Struct|BreakMinimalViewInfo _desiredview)))
  (Variables|Default|SetFloorLocation (Transformation|GetActorLocation (Variables|Default|GetFloor)))
  (Variables|Default|SetZ (- (.Z (Math|Vector|BreakVector (Variables|Default|GetCameraLocation))) (.Z (Math|Vector|BreakVector (Variables|Default|GetFloorLocation)))))
  (bind _output_get (Variables|Default|SetFrustrumHeight (* (Math|Trig|Tan(Radians) (Math|Trig|DegreesToRadians (/ (Variables|/Script/Engine.CameraComponent|GetFieldOfView (Variables|Default|GetCamera)) 2.0))) (- (.Z (Math|Vector|BreakVector (Variables|Default|GetCameraLocation))) (.Z (Math|Vector|BreakVector (Variables|Default|GetFloorLocation)))))))
  (Variables|Default|SetFrustrumWidth (* _output_get (Variables|/Script/Engine.CameraComponent|GetAspectRatio (Variables|Default|GetCamera)))))

(fn GetFOVCorners
  (bind _playerlocation (Variables|Default|GetPlayerLocation))
  (bind _posmultiplier (LocalVariables|GetPosMultiplier))
  (bind (_x _y) (Math|Vector|BreakVector _playerlocation))
  (LocalVariables|SetNegMultiplier (* (LocalVariables|GetPosMultiplier) -1.0))
  (LocalVariables|SetPlayerVec2D (Math|Vector|MakeVector _x _y 0.0))
  (Variables|Default|SetUpperLeft (+ (Math|Vector|MakeVector (/ (Variables|Default|GetFrustrumHeight) (LocalVariables|GetPosMultiplier)) (/ (Variables|Default|GetFrustrumWidth) (LocalVariables|GetNegMultiplier)) 1.5e+02) (Variables|Default|GetFloorLocation) (LocalVariables|GetPlayerVec2D)))
  (Variables|Default|SetUpperRight (+ (Math|Vector|MakeVector (/ (Variables|Default|GetFrustrumHeight) _posmultiplier) (/ (Variables|Default|GetFrustrumWidth) _posmultiplier) 1.5e+02) (Variables|Default|GetFloorLocation) (LocalVariables|GetPlayerVec2D)))
  (Variables|Default|SetBottomLeft (+ (Math|Vector|MakeVector (/ (Variables|Default|GetFrustrumHeight) (LocalVariables|GetNegMultiplier)) (/ (Variables|Default|GetFrustrumWidth) (LocalVariables|GetNegMultiplier)) 1.5e+02) (Variables|Default|GetFloorLocation) (LocalVariables|GetPlayerVec2D)))
  (Variables|Default|SetBottomRight (+ (Math|Vector|MakeVector (/ (Variables|Default|GetFrustrumHeight) (LocalVariables|GetNegMultiplier)) (/ (Variables|Default|GetFrustrumWidth) (LocalVariables|GetPosMultiplier)) 1.5e+02) (Variables|Default|GetFloorLocation) (LocalVariables|GetPlayerVec2D))))

(fn GetRandPointonPerim
  (bind _bottomleft (Variables|Default|GetBottomLeft))
  (bind _bottomright (Variables|Default|GetBottomRight))
  (bind _upperleft (Variables|Default|GetUpperLeft))
  (bind _upperright (Variables|Default|GetUpperRight))
  (bind (_x _y _z) (Math|Vector|BreakVector _upperleft))
  (bind (_x_2 _y_2 _z_2) (Math|Vector|BreakVector _upperright))
  (bind (_x_3 _y_3 _z_3) (Math|Vector|BreakVector _bottomleft))
  (bind (_x_4 _y_4 _z_4) (Math|Vector|BreakVector _bottomright))
  (bind _output_get (Variables|Default|SetEdge (Math|Random|RandomIntegerinRange 0 3)))
  (switch int _output_get
    (:0
      (return (Math|Vector|MakeVector (Math|Random|RandomFloatinRange _x_4 _x_2) _y_2 _z_2)))
    (:1
      (return (Math|Vector|MakeVector _x_4 (Math|Random|RandomFloatinRange _y_3 _y_4) _z_4)))
    (:2
      (return (Math|Vector|MakeVector (Math|Random|RandomFloatinRange _x_3 _x) _y_3 _z_3)))
    (:3
      (return (Math|Vector|MakeVector _x (Math|Random|RandomFloatinRange _y (.Y (Math|Vector|BreakVector (Variables|Default|GetUpperRight)))) _z)))))