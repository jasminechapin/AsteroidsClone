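; Asteroid for a twin-stick shooter that crosses the camera's view and breaks apart when shot.
; On BeginPlay it builds a view rectangle from camera FOV and aspect ratio, then teleports to a random perimeter point.
; It moves its mesh toward a second perimeter point over a fixed time, then destroys itself.
; A TwinStickProjectile hit spawns two offset AsteroidPieces, pushing only the first, increases the player's score and destroys the asteroid.
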(event EventBeginPlay
  (CallFunction|GetFOVDimensions)
  (CallFunction|GetFOVCorners)
  (bind _randposn (CallFunction|GetRandPointonPerim))
  (Transformation|SetActorLocation _randposn false true)
  (bind _randposn_2 (CallFunction|GetRandPointonPerim))
  (Utilities|FlowControl|Sequence
    (:then_0
      (Components|MoveComponentTo (Variables|Debug|GetStaticMeshComponent) _randposn_2 "0, 0, 0" false false 5.0 false)
      (Actor|DestroyActor))))

(event Collision|EventHit
  (params (MyComp :type Primitive%20Component%20Object%20Reference) (Other :type Actor%20Object%20Reference) (OtherComp :type Primitive%20Component%20Object%20Reference) (bSelfMoved :type Boolean) (HitLocation :type Vector :default "0, 0, 0") (HitNormal :type Vector :default "0, 0, 0") (NormalImpulse :type Vector :default "0, 0, 0") (Hit :type Hit%20Result%20Structure%20%28by%20ref%29))
  (Utilities|Casting|CastToTwinStickProjectile Other)
  (Utilities|FlowControl|Sequence
    (:then_0
      (bind _returnvalue (Game|SpawnActorfromClass "/Game/Blueprints/AsteroidPiece.AsteroidPiece_C" (Math|Transform|MakeTransform (+ HitLocation "30.000000,30.000000,0.000000")) "AdjustIfPossibleButAlwaysSpawn" 0 0))
      (Physics|AddImpulse (Variables|/Game/Blueprints/AsteroidPiece.AsteroidPiece_C|GetCapsule _returnvalue) HitNormal "None" true)
      (Variables|/Game/Blueprints/AsteroidPiece.AsteroidPiece_C|SetVelocity _returnvalue (stale EventBeginPlay _randposn_2)))
    (:then_1
      (Game|SpawnActorfromClass "/Game/Blueprints/AsteroidPiece.AsteroidPiece_C" (Math|Transform|MakeTransform (- HitLocation "30.000000,30.000000, 0")) "AdjustIfPossibleButAlwaysSpawn" 0 0))
    (:then_2
      (bind _astwin_stick_pawn (Utilities|Casting|CastToTwinStickPawn (Game|Player|GetPlayerPawn 0)))
      (Default|IncreaseScore _astwin_stick_pawn)
      (Actor|DestroyActor))))

(fn ConstructionScript)

(fn GetFOVDimensions
  (bind _returnvalue (Game|GetPlayerCameraManager 0))
  (Variables|Default|SetCameraLocation (Camera|GetCameraLocation _returnvalue))
  (bind _astwin_stick_pawn (Utilities|Casting|CastToTwinStickPawn (Game|Player|GetPlayerPawn 0)))
  (bind _output_get (Variables|Default|SetFrustrumHeight (* (Math|Trig|Tan(Radians) (Math|Trig|DegreesToRadians (/ (Camera|GetFOVAngle _returnvalue) 2.0))) 2.1e+03)))
  (Variables|Default|SetFrustrumWidth (* _output_get (Variables|/Script/Engine.PlayerCameraManager|GetDefaultAspectRatio (Game|GetPlayerCameraManager 0)))))

(fn GetFOVCorners
  (bind _posmultiplier (LocalVariables|GetPosMultiplier))
  (LocalVariables|SetNegMultiplier (* (LocalVariables|GetPosMultiplier) -1.0))
  (Variables|Default|SetUpperLeft (+ (Math|Vector|MakeVector (/ (Variables|Default|GetFrustrumHeight) (LocalVariables|GetPosMultiplier)) (/ (Variables|Default|GetFrustrumWidth) (LocalVariables|GetNegMultiplier)) 1.6e+02) (Variables|Default|GetFloorLocation)))
  (Variables|Default|SetUpperRight (+ (Math|Vector|MakeVector (/ (Variables|Default|GetFrustrumHeight) _posmultiplier) (/ (Variables|Default|GetFrustrumWidth) _posmultiplier) 1.6e+02) (Variables|Default|GetFloorLocation)))
  (Variables|Default|SetBottomLeft (+ (Math|Vector|MakeVector (/ (Variables|Default|GetFrustrumHeight) (LocalVariables|GetNegMultiplier)) (/ (Variables|Default|GetFrustrumWidth) (LocalVariables|GetNegMultiplier)) 1.6e+02) (Variables|Default|GetFloorLocation)))
  (Variables|Default|SetBottomRight (+ (Math|Vector|MakeVector (/ (Variables|Default|GetFrustrumHeight) 1.0) (/ (Variables|Default|GetFrustrumWidth) (LocalVariables|GetPosMultiplier)) 1.6e+02) (Variables|Default|GetFloorLocation))))

(fn GetRandPointonPerim
  (bind _bottomleft (Variables|Default|GetBottomLeft))
  (bind _bottomright (Variables|Default|GetBottomRight))
  (bind _upperleft (Variables|Default|GetUpperLeft))
  (bind _upperright (Variables|Default|GetUpperRight))
  (bind (_x _y _z) (Math|Vector|BreakVector _upperleft))
  (bind (_x_2 _y_2 _z_2) (Math|Vector|BreakVector _upperright))
  (bind (_x_3 _y_3 _z_3) (Math|Vector|BreakVector _bottomleft))
  (bind (_x_4 _y_4 _z_4) (Math|Vector|BreakVector _bottomright))
  (bind _output_get (Variables|Default|SetEdge (Math|Random|RandomIntegerinRange 0 3)))
  (switch int _output_get
    (:0
      (return (Math|Vector|MakeVector (Math|Random|RandomFloatinRange _x_4 _x_2) _y_2 _z_2)))
    (:1
      (return (Math|Vector|MakeVector _x_4 (Math|Random|RandomFloatinRange _y_3 _y_4) _z_4)))
    (:2
      (return (Math|Vector|MakeVector (Math|Random|RandomFloatinRange _x_3 _x) _y_3 _z_3)))
    (:3
      (return (Math|Vector|MakeVector _x (Math|Random|RandomFloatinRange _y (.Y (Math|Vector|BreakVector (Variables|Default|GetUpperRight)))) _z)))))